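; BP_PU_FOUR is an oven ("four") that flags pizzas as heating while they sit inside its Zone_Four trigger.
; On overlap begin and end, it searches all BP_PU_Pizza actors for the overlapping one and sets its Chauffe flag true or false.
; Pickup and Drop events, called by BP_MotionController, are empty here; their physics and attach/detach logic is left disconnected, so the oven does not respond to grabbing.
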(event `/Game/Pizza/Blueprints/Base/PickupActorInterface.Pickup`
  (params (AttachTo :type "SceneComponent Object Reference")))

(event `/Game/Pizza/Blueprints/Base/PickupActorInterface.Drop`)

(event `self.Zone_Four.OnComponentBeginOverlap`
  (params (OverlappedComponent :type "PrimitiveComponent Object Reference") (OtherActor :type "Actor Object Reference") (OtherComp :type "PrimitiveComponent Object Reference") (OtherBodyIndex :type Integer) (bFromSweep :type Boolean) (SweepResult :type "HitResult Structure (by ref)"))
  (bind _outactors (`GameplayStatics.GetAllActorsOfClass` "/Game/Pizza/Blueprints/BP_PU_Pizza.BP_PU_Pizza_C"))
  (for _array_element _outactors
    (if (== _array_element OtherActor)
      (bind _asbp_pu_pizza (cast `/Game/Pizza/Blueprints/BP_PU_Pizza` OtherActor))
      (set `/Game/Pizza/Blueprints/BP_PU_Pizza.Chauffe` true _asbp_pu_pizza))))

(event `self.Zone_Four.OnComponentEndOverlap`
  (params (OverlappedComponent :type "PrimitiveComponent Object Reference") (OtherActor :type "Actor Object Reference") (OtherComp :type "PrimitiveComponent Object Reference") (OtherBodyIndex :type Integer))
  (bind _outactors (`GameplayStatics.GetAllActorsOfClass` "/Game/Pizza/Blueprints/BP_PU_Pizza.BP_PU_Pizza_C"))
  (for _array_element _outactors
    (if (== _array_element OtherActor)
      (bind _asbp_pu_pizza (cast `/Game/Pizza/Blueprints/BP_PU_Pizza` OtherActor))
      (set `/Game/Pizza/Blueprints/BP_PU_Pizza.Chauffe` false _asbp_pu_pizza))))

(fn `UserConstructionScript`)