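; Pickable pizza actor, grabbed via BP_MotionController, that gets topped, cooked or thrown away.
; Overlapping ingredients are destroyed and revealed as meshes on the raw pizza; one sauce type (soap included) stacks through three levels, only before toppings.
; While Chauffe is set, Tick accumulates heat, triggering cooked and burnt material swaps, with a further disintegration threshold.
; Touching BP_Poubelle increments its food counter, then destroys the pizza after a delay.
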(event OnComponentBeginOverlap(Collider)
  (params (OverlappedComponent :type Primitive%20Component%20Object%20Reference) (OtherActor :type Actor%20Object%20Reference) (OtherComp :type Primitive%20Component%20Object%20Reference) (OtherBodyIndex :type Integer) (bFromSweep :type Boolean) (SweepResult :type Hit%20Result%20Structure%20%28by%20ref%29))
  (bind _etat_sauce_3 (Variables|Default|GetEtat%20Sauce%203))
  (bind _etat_savon (Variables|Default|GetEtat%20Savon))
  (bind _etat_sauce_2 (Variables|Default|GetEtat%20Sauce%202))
  (if (Rendering|IsVisible (Variables|/Script/Engine.Actor|GetRootComponent OtherActor))
    (if (not (or (Variables|Default|GetCuite) (Variables|Default|GetBrulée)))
      (if (== (Utilities|GetClass OtherActor) "/Game/Pizza/Blueprints/Garnitures/BP_PU_Fromage.BP_PU_Fromage_C")
        (if (not (Variables|Default|GetFromage))
          ;[1 0.9209 0] Ajout Fromage
          (bind _outactors (Actor|GetAllActorsOfClass "/Game/Pizza/Blueprints/Garnitures/BP_PU_Fromage.BP_PU_Fromage_C"))
          (for _array_element _outactors
            (if (== _array_element OtherActor)
              (Rendering|SetVisibility (Variables|Default|GetEtat%20Fromage) true false)
              (Variables|Default|SetFromage true)
              (Variables|Default|SetGarnitureON true)
              (bind _asbp_pu_fromage (Utilities|Casting|CastToBP_PU_Fromage OtherActor))
              (bind _output_get (Variables|Default|SetFromage_Cell _asbp_pu_fromage))
              (Rendering|SetVisibility (Variables|/Script/Engine.Actor|GetRootComponent (stale _output_get_2)) false false)
              (Actor|DestroyActor OtherActor))))
        (elif (== (Utilities|GetClass OtherActor) "/Game/Pizza/Blueprints/Garnitures/BP_PU_Sauce.BP_PU_Sauce_C")
          (if (not (Variables|Default|GetSauce%202))
            (if (not (Variables|Default|GetSauce%203))
              (if (not (Variables|Default|GetSavon))
                (if (not (Variables|Default|GetGarnitureON))
                  ;[1 0.04338 0] Sauce 1 : Rouge
                  (bind _outactors_2 (Actor|GetAllActorsOfClass "/Game/Pizza/Blueprints/Garnitures/BP_PU_Sauce.BP_PU_Sauce_C"))
                  (for _array_element_2 _outactors_2
                    (if (== _array_element_2 OtherActor)
                      (Variables|Default|SetNiveau%20Sauce (+ 1 (Variables|Default|GetNiveau%20Sauce)))
                      (if (== (Variables|Default|GetNiveau%20Sauce) 1)
                        (Audio|PlaySound2D "/Game/Pizza/SONS/Splash3_Cue.Splash3_Cue" 1.0 1.0 0.0 0 0)
                        (Rendering|SetVisibility (Variables|Default|GetEtat%20Sauce%201) true false)
                        (Components|StaticMesh|SetStaticMesh (Variables|Default|GetEtat%20Sauce%201) "/Game/Pizza/Models_3D/Garnitures/Sauces/sauce_T1_Sphere001.sauce_T1_Sphere001")
                        (Variables|Default|SetSauce%20Niv1 true)
                        (bind _asbp_pu_sauce (Utilities|Casting|CastToBP_PU_Sauce OtherActor :!label _label))
                        (bind _output_get_2 (Variables|Default|SetSauce1_Cell _asbp_pu_sauce))
                        (bind _outactors_3 (Actor|GetAllActorsOfClass "/Game/Pizza/Blueprints/BP_PU_Dépot.BP_PU_Dépot_C"))
                        (for _array_element_3 _outactors_3
                          (Utilities|Casting|CastToBP_PU_Dépot _array_element_3)
                          (Rendering|SetVisibility (Variables|/Script/Engine.Actor|GetRootComponent _output_get_2) false false)
                          (Actor|DestroyActor OtherActor))
                        (elif (== (Variables|Default|GetNiveau%20Sauce) 2)
                          (Audio|PlaySound2D "/Game/Pizza/SONS/Splash1_Cue.Splash1_Cue" 1.0 1.0 0.0 0 0)
                          (Components|StaticMesh|SetStaticMesh (Variables|Default|GetEtat%20Sauce%201) "/Game/Pizza/Models_3D/Garnitures/Sauces/sauce_T2_Sphere001.sauce_T2_Sphere001")
                          (Variables|Default|SetSauce%20Niv2 true)
                          (Variables|Default|SetSauce%201 true :!label _label_2)
                          (goto _label)
                          (elif (>= (Variables|Default|GetNiveau%20Sauce) 3)
                            (Audio|PlaySound2D "/Game/Pizza/SONS/Splash3_Cue.Splash3_Cue" 1.0 1.0 0.0 0 0)
                            (Components|StaticMesh|SetStaticMesh (Variables|Default|GetEtat%20Sauce%201) "/Game/Pizza/Models_3D/Garnitures/Sauces/sauce_T3_Cylinder002.sauce_T3_Cylinder002")
                            (Variables|Default|SetSauce%20Niv3 true)
                            (goto _label_2))))))))))
          (elif (== (Utilities|GetClass OtherActor) "/Game/Pizza/Blueprints/Garnitures/BP_PU_Sauce2.BP_PU_Sauce2_C")
            (if (not (Variables|Default|GetSauce%201))
              (if (not (Variables|Default|GetSauce%203))
                (if (not (Variables|Default|GetSavon))
                  ;[0 0.3125 0.02821] Sauce 2: Verte
                  (if (not (Variables|Default|GetGarnitureON))
                    (bind _outactors_4 (Actor|GetAllActorsOfClass "/Game/Pizza/Blueprints/Garnitures/BP_PU_Sauce2.BP_PU_Sauce2_C"))
                    (for _array_element_4 _outactors_4
                      (if (== _array_element_4 OtherActor)
                        (Variables|Default|SetNiveau%20Sauce (+ 1 (Variables|Default|GetNiveau%20Sauce)))
                        (if (== (Variables|Default|GetNiveau%20Sauce) 1)
                          (Audio|PlaySound2D "/Game/Pizza/SONS/Splash3_Cue.Splash3_Cue" 1.0 1.0 0.0 0 0)
                          (Rendering|SetVisibility (Variables|Default|GetEtat%20Sauce%202) true false)
                          (Components|StaticMesh|SetStaticMesh _etat_sauce_2 "/Game/Pizza/Models_3D/Garnitures/Sauces/sauce_T1_Sphere001.sauce_T1_Sphere001")
                          (Variables|Default|SetSauce%20Niv1 true)
                          (Variables|Default|SetSauce%202 true :!label _label_3)
                          (bind _asbp_pu_sauce_2 (Utilities|Casting|CastToBP_PU_Sauce2 OtherActor))
                          (bind _output_get_3 (Variables|Default|SetSauce1_Cell _asbp_pu_sauce_2))
                          (bind _outactors_5 (Actor|GetAllActorsOfClass "/Game/Pizza/Blueprints/BP_PU_Dépot.BP_PU_Dépot_C"))
                          (for _array_element_5 _outactors_5
                            (Utilities|Casting|CastToBP_PU_Dépot _array_element_5)
                            (Rendering|SetVisibility (Variables|/Script/Engine.Actor|GetRootComponent _output_get_2) false false)
                            (Actor|DestroyActor OtherActor))
                          (elif (== (Variables|Default|GetNiveau%20Sauce) 2)
                            (Audio|PlaySound2D "/Game/Pizza/SONS/Splash1_Cue.Splash1_Cue" 1.0 1.0 0.0 0 0)
                            (Components|StaticMesh|SetStaticMesh _etat_sauce_2 "/Game/Pizza/Models_3D/Garnitures/Sauces/sauce_T2_Sphere001.sauce_T2_Sphere001")
                            (Variables|Default|SetSauce%20Niv2 true)
                            (goto _label_3)
                            (elif (>= (Variables|Default|GetNiveau%20Sauce) 3)
                              (Audio|PlaySound2D "/Game/Pizza/SONS/Splash3_Cue.Splash3_Cue" 1.0 1.0 0.0 0 0)
                              (Components|StaticMesh|SetStaticMesh _etat_sauce_2 "/Game/Pizza/Models_3D/Garnitures/Sauces/sauce_T3_Cylinder002.sauce_T3_Cylinder002")
                              (Variables|Default|SetSauce%20Niv3 true)
                              (goto _label_3))))))))))
            (elif (== (Utilities|GetClass OtherActor) "/Game/Pizza/Blueprints/Garnitures/BP_PU_Sauce3.BP_PU_Sauce3_C")
              (if (not (Variables|Default|GetSauce%201))
                (if (not (Variables|Default|GetSauce%202))
                  (if (not (Variables|Default|GetSavon))
                    (if (not (Variables|Default|GetGarnitureON))
                      ;[1 0.2186 0] Sauce 3: Orange
                      (bind _outactors_6 (Actor|GetAllActorsOfClass "/Game/Pizza/Blueprints/Garnitures/BP_PU_Sauce3.BP_PU_Sauce3_C"))
                      (for _array_element_6 _outactors_6
                        (if (== _array_element_6 OtherActor)
                          (Variables|Default|SetNiveau%20Sauce (+ 1 (Variables|Default|GetNiveau%20Sauce)))
                          (if (== (Variables|Default|GetNiveau%20Sauce) 1)
                            (Audio|PlaySound2D "/Game/Pizza/SONS/Splash3_Cue.Splash3_Cue" 1.0 1.0 0.0 0 0)
                            (Rendering|SetVisibility _etat_sauce_3 true false)
                            (Components|StaticMesh|SetStaticMesh _etat_sauce_3 "/Game/Pizza/Models_3D/Garnitures/Sauces/sauce_T1_Sphere001.sauce_T1_Sphere001")
                            (Variables|Default|SetSauce%20Niv1 true)
                            (Variables|Default|SetSauce%203 true :!label _label_4)
                            (bind _asbp_pu_sauce_3 (Utilities|Casting|CastToBP_PU_Sauce3 OtherActor))
                            (bind _output_get_4 (Variables|Default|SetSauce1_Cell _asbp_pu_sauce_3))
                            (bind _outactors_7 (Actor|GetAllActorsOfClass "/Game/Pizza/Blueprints/BP_PU_Dépot.BP_PU_Dépot_C"))
                            (for _array_element_7 _outactors_7
                              (Utilities|Casting|CastToBP_PU_Dépot _array_element_7)
                              (Rendering|SetVisibility (Variables|/Script/Engine.Actor|GetRootComponent _output_get_2) false false)
                              (Actor|DestroyActor OtherActor))
                            (elif (== (Variables|Default|GetNiveau%20Sauce) 2)
                              (Audio|PlaySound2D "/Game/Pizza/SONS/Splash1_Cue.Splash1_Cue" 1.0 1.0 0.0 0 0)
                              (Components|StaticMesh|SetStaticMesh _etat_sauce_3 "/Game/Pizza/Models_3D/Garnitures/Sauces/sauce_T2_Sphere001.sauce_T2_Sphere001")
                              (Variables|Default|SetSauce%20Niv2 true)
                              (goto _label_4)
                              (elif (>= (Variables|Default|GetNiveau%20Sauce) 3)
                                (Audio|PlaySound2D "/Game/Pizza/SONS/Splash3_Cue.Splash3_Cue" 1.0 1.0 0.0 0 0)
                                (Components|StaticMesh|SetStaticMesh _etat_sauce_3 "/Game/Pizza/Models_3D/Garnitures/Sauces/sauce_T3_Cylinder002.sauce_T3_Cylinder002")
                                (Variables|Default|SetSauce%20Niv3 true)
                                (goto _label_4))))))))))
              (elif (== (Utilities|GetClass OtherActor) "/Game/Pizza/Blueprints/Garnitures/BP_PU_Savon.BP_PU_Savon_C")
                (if (not (Variables|Default|GetSauce%201))
                  (if (not (Variables|Default|GetSauce%202))
                    (if (not (Variables|Default|GetSauce%203))
                      ;[1 0.3352 0.7278] Savon
                      (if (not (Variables|Default|GetGarnitureON))
                        (bind _outactors_8 (Actor|GetAllActorsOfClass "/Game/Pizza/Blueprints/Garnitures/BP_PU_Savon.BP_PU_Savon_C"))
                        (for _array_element_8 _outactors_8
                          (if (== _array_element_8 OtherActor)
                            (Variables|Default|SetNiveau%20Sauce (+ 1 (Variables|Default|GetNiveau%20Sauce)))
                            (if (== (Variables|Default|GetNiveau%20Sauce) 1)
                              (Audio|PlaySound2D "/Game/Pizza/SONS/Splash3_Cue.Splash3_Cue" 1.0 1.0 0.0 0 0)
                              (Rendering|SetVisibility _etat_savon true false)
                              (Components|StaticMesh|SetStaticMesh _etat_savon "/Game/Pizza/Models_3D/Garnitures/Sauces/sauce_T1_Sphere001.sauce_T1_Sphere001")
                              (Variables|Default|SetSauce%20Niv1 true)
                              (Variables|Default|SetSavon true :!label _label_5)
                              (bind _asbp_pu_savon (Utilities|Casting|CastToBP_PU_Savon OtherActor))
                              (bind _output_get_5 (Variables|Default|SetSavon%20Cell _asbp_pu_savon))
                              (bind _outactors_9 (Actor|GetAllActorsOfClass "/Game/Pizza/Blueprints/BP_PU_Dépot.BP_PU_Dépot_C"))
                              (for _array_element_9 _outactors_9
                                (Rendering|SetVisibility (Variables|/Script/Engine.Actor|GetRootComponent _output_get_2) false false)
                                (Actor|DestroyActor OtherActor))
                              (elif (== (Variables|Default|GetNiveau%20Sauce) 2)
                                (Audio|PlaySound2D "/Game/Pizza/SONS/Splash1_Cue.Splash1_Cue" 1.0 1.0 0.0 0 0)
                                (Components|StaticMesh|SetStaticMesh _etat_savon "/Game/Pizza/Models_3D/Garnitures/Sauces/sauce_T2_Sphere001.sauce_T2_Sphere001")
                                (Variables|Default|SetSauce%20Niv2 true)
                                (goto _label_5)
                                (elif (>= (Variables|Default|GetNiveau%20Sauce) 3)
                                  (Audio|PlaySound2D "/Game/Pizza/SONS/Splash3_Cue.Splash3_Cue" 1.0 1.0 0.0 0 0)
                                  (Components|StaticMesh|SetStaticMesh _etat_savon "/Game/Pizza/Models_3D/Garnitures/Sauces/sauce_T3_Cylinder002.sauce_T3_Cylinder002")
                                  (Variables|Default|SetSauce%20Niv3 true)
                                  (goto _label_5))))))))))
                (elif (== (Utilities|GetClass OtherActor) "/Game/Pizza/Blueprints/Garnitures/BP_PU_Champi.BP_PU_Champi_C")
                  ;[1 0.3344 0.1028] Champignon
                  (if (not (Variables|Default|GetChampignon))
                    (bind _outactors_10 (Actor|GetAllActorsOfClass "/Game/Pizza/Blueprints/Garnitures/BP_PU_Champi.BP_PU_Champi_C"))
                    (for _array_element_10 _outactors_10
                      (if (== _array_element_10 OtherActor)
                        (Rendering|SetVisibility (Variables|Default|GetEtat%20Champi) true false)
                        (Variables|Default|SetChampignon true)
                        (Variables|Default|SetGarnitureON true)
                        (bind _asbp_pu_champi (Utilities|Casting|CastToBP_PU_Champi OtherActor))
                        (bind _output_get_6 (Variables|Default|SetChampignon_Cell _asbp_pu_champi))
                        (Rendering|SetVisibility (Variables|/Script/Engine.Actor|GetRootComponent _output_get_2) false false)
                        (Actor|DestroyActor OtherActor))))
                  (elif (== (Utilities|GetClass OtherActor) "/Game/Pizza/Blueprints/Garnitures/BP_PU_Chorizo.BP_PU_Chorizo_C")
                    ;[1 0.1409 0.08121] Chorizo
                    (if (not (Variables|Default|GetChorizo))
                      (bind _outactors_11 (Actor|GetAllActorsOfClass "/Game/Pizza/Blueprints/Garnitures/BP_PU_Chorizo.BP_PU_Chorizo_C"))
                      (for _array_element_11 _outactors_11
                        (if (== _array_element_11 OtherActor)
                          (Rendering|SetVisibility (Variables|Default|GetEtat%20Chorizo) true false)
                          (Variables|Default|SetChorizo true)
                          (Variables|Default|SetGarnitureON true)
                          (bind _asbp_pu_chorizo (Utilities|Casting|CastToBP_PU_Chorizo OtherActor))
                          (bind _output_get_7 (Variables|Default|SetChorizo_Cell _asbp_pu_chorizo))
                          (Rendering|SetVisibility (Variables|/Script/Engine.Actor|GetRootComponent _output_get_2) false false)
                          (Actor|DestroyActor OtherActor))))
                    (elif (== (Utilities|GetClass OtherActor) "/Game/Pizza/Blueprints/Garnitures/BP_PU_Poivron.BP_PU_Poivron_C")
                      ;[0 1 0.02053] Poivron
                      (if (not (Variables|Default|GetPoivron))
                        (bind _outactors_12 (Actor|GetAllActorsOfClass "/Game/Pizza/Blueprints/Garnitures/BP_PU_Poivron.BP_PU_Poivron_C"))
                        (for _array_element_12 _outactors_12
                          (if (== _array_element_12 OtherActor)
                            (Rendering|SetVisibility (Variables|Default|GetEtat%20Poivron) true false)
                            (Variables|Default|SetPoivron true)
                            (Variables|Default|SetGarnitureON true)
                            (bind _asbp_pu_poivron (Utilities|Casting|CastToBP_PU_Poivron OtherActor))
                            (bind _output_get_8 (Variables|Default|SetPoivron_Cell _asbp_pu_poivron))
                            (Rendering|SetVisibility (Variables|/Script/Engine.Actor|GetRootComponent _output_get_2) false false)
                            (Actor|DestroyActor OtherActor))))
                      (elif (== (Utilities|GetClass OtherActor) "/Game/Pizza/Blueprints/Garnitures/BP_PU_DECHET.BP_PU_DECHET_C")
                        ;[0.2917 0.2917 0.2917] Dechet
                        (if (not (Variables|Default|GetDechet))
                          (bind _outactors_13 (Actor|GetAllActorsOfClass "/Game/Pizza/Blueprints/Garnitures/BP_PU_DECHET.BP_PU_DECHET_C"))
                          (for _array_element_13 _outactors_13
                            (if (== _array_element_13 OtherActor)
                              (Rendering|SetVisibility (Variables|Default|GetEtat%20Dechet) true false)
                              (Variables|Default|SetDechet true)
                              (Variables|Default|SetGarnitureON true)
                              (bind _asbp_pu_dechet (Utilities|Casting|CastToBP_PU_DECHET OtherActor))
                              (bind _output_get_9 (Variables|Default|SetDechet%20Cell _asbp_pu_dechet))
                              (Rendering|SetVisibility (Variables|/Script/Engine.Actor|GetRootComponent _output_get_2) false false)
                              (Actor|DestroyActor OtherActor))))
                        (elif (== (Utilities|GetClass OtherActor) "/Game/Pizza/Blueprints/Garnitures/BP_PU_Crevettes.BP_PU_Crevettes_C")
                          ;[0.1359 0.5833 0] Crevette
                          (if (not (Variables|Default|GetCrevettes))
                            (bind _outactors_14 (Actor|GetAllActorsOfClass "/Game/Pizza/Blueprints/Garnitures/BP_PU_Crevettes.BP_PU_Crevettes_C"))
                            (for _array_element_14 _outactors_14
                              (if (== _array_element_14 OtherActor)
                                (Rendering|SetVisibility (Variables|Default|GetEtat%20Crevettes) true false)
                                (Variables|Default|SetCrevettes true)
                                (Variables|Default|SetGarnitureON true)
                                (bind _asbp_pu_crevettes (Utilities|Casting|CastToBP_PU_Crevettes OtherActor))
                                (bind _output_get_10 (Variables|Default|SetCrevette%20Cell _asbp_pu_crevettes))
                                (Rendering|SetVisibility (Variables|/Script/Engine.Actor|GetRootComponent _output_get_2) false false)
                                (Actor|DestroyActor OtherActor))))
                          (elif (== (Utilities|GetClass OtherActor) "/Game/Pizza/Blueprints/Garnitures/BP_PU_Ver.BP_PU_Ver_C")
                            ;[0.5833 0.4438 0.1276] Ver
                            (if (not (Variables|Default|GetVer))
                              (bind _outactors_15 (Actor|GetAllActorsOfClass "/Game/Pizza/Blueprints/Garnitures/BP_PU_Ver.BP_PU_Ver_C"))
                              (for _array_element_15 _outactors_15
                                (if (== _array_element_15 OtherActor)
                                  (Rendering|SetVisibility (Variables|Default|GetEtat%20Ver) true false)
                                  (Variables|Default|SetVer true)
                                  (Variables|Default|SetGarnitureON true)
                                  (bind _asbp_pu_ver (Utilities|Casting|CastToBP_PU_Ver OtherActor))
                                  (bind _output_get_11 (Variables|Default|SetVer%20Cell _asbp_pu_ver))
                                  (Rendering|SetVisibility (Variables|/Script/Engine.Actor|GetRootComponent _output_get_2) false false)
                                  (Actor|DestroyActor OtherActor))))
                            (elif (== (Utilities|GetClass OtherActor) "/Game/Pizza/Blueprints/Garnitures/BP_PU_Moisi.BP_PU_Moisi_C")
                              ;[0.1628 0.5833 0.2145] Moisi
                              (if (not (Variables|Default|GetMoisi))
                                (bind _outactors_16 (Actor|GetAllActorsOfClass "/Game/Pizza/Blueprints/Garnitures/BP_PU_Moisi.BP_PU_Moisi_C"))
                                (for _array_element_16 _outactors_16
                                  (if (== _array_element_16 OtherActor)
                                    (Rendering|SetVisibility (Variables|Default|GetEtat%20Moisi) true false)
                                    (Variables|Default|SetMoisi true)
                                    (Variables|Default|SetGarnitureON true)
                                    (bind _asbp_pu_moisi (Utilities|Casting|CastToBP_PU_Moisi OtherActor))
                                    (bind _output_get_12 (Variables|Default|SetMoisi%20Cell _asbp_pu_moisi))
                                    (Rendering|SetVisibility (Variables|/Script/Engine.Actor|GetRootComponent _output_get_2) false false)
                                    (Actor|DestroyActor OtherActor)))))))))))))))))))

(event OnComponentBeginOverlap(StaticMeshComponent)
  (params (OverlappedComponent :type Primitive%20Component%20Object%20Reference) (OtherActor :type Actor%20Object%20Reference) (OtherComp :type Primitive%20Component%20Object%20Reference) (OtherBodyIndex :type Integer) (bFromSweep :type Boolean) (SweepResult :type Hit%20Result%20Structure%20%28by%20ref%29))
  (bind _asbp_poubelle (Utilities|Casting|CastToBP_Poubelle OtherActor))
  (if (stale _bsuccess)
    (Variables|/Game/Pizza/Blueprints/Poubelle/BP_Poubelle.BP_Poubelle_C|SetCOMPTEUR%20BOUFFE _asbp_poubelle (+ (Variables|/Game/Pizza/Blueprints/Poubelle/BP_Poubelle.BP_Poubelle_C|GetCOMPTEUR%20BOUFFE _asbp_poubelle) 1))
    (Utilities|FlowControl|Delay 2.0)
    (Actor|DestroyActor)))

(event Custom|Vendu
  ;[0 1 0.02272] VENDU
)

(event Custom|CUIT
  (bind _etat_ver (Variables|Default|GetEtat%20Ver))
  ;[1 0.04731 0] CUISSON
  (Rendering|Material|SetMaterial (Variables|Debug|GetStaticMeshComponent) 0 "/Game/Pizza/Mat/MAT_Pizza_Cuit.MAT_Pizza_Cuit")
  (Rendering|Material|SetMaterial (Variables|Default|GetEtat%20Sauce%201) 0 "/Game/Pizza/Models_3D/Garnitures/Sauces/MAT_Sauce1_Cuite.MAT_Sauce1_Cuite")
  (Rendering|Material|SetMaterial (Variables|Default|GetEtat%20Sauce%202) 0 "/Game/Pizza/Models_3D/Garnitures/Sauces/MAT_Sauce2_Cuite.MAT_Sauce2_Cuite")
  (Rendering|Material|SetMaterial (Variables|Default|GetEtat%20Savon) 0 "/Game/Pizza/Models_3D/Garnitures/Sauces/MAT_Savon_Cuit.MAT_Savon_Cuit")
  (Rendering|Material|SetMaterial (Variables|Default|GetEtat%20Sauce%203) 0 "/Game/Pizza/Models_3D/Garnitures/Sauces/MAT_Sauce3_Cuite.MAT_Sauce3_Cuite")
  (Rendering|Material|SetMaterial (Variables|Default|GetEtat%20Champi) 0 "/Game/Pizza/Models_3D/Garnitures/Champis/Mat_Champi_Cuit.Mat_Champi_Cuit")
  (Rendering|Material|SetMaterial (Variables|Default|GetEtat%20Chorizo) 0 "/Game/Pizza/Models_3D/Garnitures/Chorizos/Mat_Chorizo_Cuit.Mat_Chorizo_Cuit")
  (Rendering|Material|SetMaterial (Variables|Default|GetEtat%20Chorizo) 1 "/Game/Pizza/Models_3D/Garnitures/Chorizos/Mat_Chorizo_+_2.Mat_Chorizo_+_2")
  (Rendering|Material|SetMaterial (Variables|Default|GetEtat%20Poivron) 0 "/Game/Pizza/Models_3D/Garnitures/Poivrons/Poivron_B_Cuit.Poivron_B_Cuit")
  (Rendering|Material|SetMaterial (Variables|Default|GetEtat%20Poivron) 1 "/Game/Pizza/Models_3D/Garnitures/Poivrons/Poivron_R_Cuit.Poivron_R_Cuit")
  (Rendering|Material|SetMaterial (Variables|Default|GetEtat%20Poivron) 2 "/Game/Pizza/Models_3D/Garnitures/Poivrons/Poivron_J_Cuit.Poivron_J_Cuit")
  (Rendering|Material|SetMaterial (Variables|Default|GetEtat%20Poivron) 3 "/Game/Pizza/Models_3D/Garnitures/Poivrons/Poivron_B_Cuit.Poivron_B_Cuit")
  (Rendering|Material|SetMaterial (Variables|Default|GetEtat%20Poivron) 4 "/Game/Pizza/Models_3D/Garnitures/Poivrons/Poivron_V_Cuit.Poivron_V_Cuit")
  (Rendering|Material|SetMaterial (Variables|Default|GetEtat%20Poivron) 5 "/Game/Pizza/Models_3D/Garnitures/Poivrons/Poivron_B_Cuit.Poivron_B_Cuit")
  (Rendering|Material|SetMaterial (Variables|Default|GetEtat%20Crevettes) 0 "/Game/Pizza/Models_3D/Garnitures/Crevettes/Mat_Crevette_Cuit.Mat_Crevette_Cuit")
  (Rendering|Material|SetMaterial (Variables|Default|GetEtat%20Crevettes) 1 "/Game/Pizza/Models_3D/Garnitures/Crevettes/Crevette2_Cuit.Crevette2_Cuit")
  (Rendering|Material|SetMaterial _etat_ver 1 "/Game/Pizza/Mat/MAT_Pizza_Cuit.MAT_Pizza_Cuit")
  (Rendering|Material|SetMaterial _etat_ver 2 "/Game/Pizza/Mat/MAT_Pizza_Cuit.MAT_Pizza_Cuit")
  (Rendering|Material|SetMaterial (Variables|Default|GetEtat%20Moisi) 0 "/Game/Pizza/Models_3D/Garnitures/Moisissure/Mat_Moisi_cuit.Mat_Moisi_cuit"))

(event Custom|BRULE
  (bind _etat_ver (Variables|Default|GetEtat%20Ver))
  ;[1 0.04731 0] CUISSON
  (Rendering|Material|SetMaterial (Variables|Default|GetEtat%20Sauce%201) 0 "/Game/Pizza/Models_3D/Garnitures/Sauces/MAT_Sauce1_Bruh.MAT_Sauce1_Bruh")
  (Rendering|Material|SetMaterial (Variables|Default|GetEtat%20Sauce%202) 0 "/Game/Pizza/Models_3D/Garnitures/Sauces/MAT_Sauce2_Bruh.MAT_Sauce2_Bruh")
  (Rendering|Material|SetMaterial (Variables|Default|GetEtat%20Savon) 0 "/Game/Pizza/Models_3D/Garnitures/Sauces/MAT_Savon_Bruh.MAT_Savon_Bruh")
  (Rendering|Material|SetMaterial (Variables|Default|GetEtat%20Sauce%203) 0 "/Game/Pizza/Models_3D/Garnitures/Sauces/MAT_Sauce3_Bruh_2.MAT_Sauce3_Bruh_2")
  (Rendering|Material|SetMaterial (Variables|Default|GetEtat%20Champi) 0 "/Game/Pizza/Models_3D/Garnitures/Champis/Mat_Champi_Bruh.Mat_Champi_Bruh")
  (Rendering|Material|SetMaterial (Variables|Default|GetEtat%20Chorizo) 0 "/Game/Pizza/Models_3D/Garnitures/Chorizos/Mat_Chorizo_Bruh.Mat_Chorizo_Bruh")
  (Rendering|Material|SetMaterial (Variables|Default|GetEtat%20Chorizo) 1 "/Game/Pizza/Models_3D/Garnitures/Chorizos/Mat_Chorizo_+_3.Mat_Chorizo_+_3")
  (Rendering|Material|SetMaterial (Variables|Default|GetEtat%20Poivron) 0 "/Game/Pizza/Models_3D/Garnitures/Poivrons/Poivron_B_Bruh.Poivron_B_Bruh")
  (Rendering|Material|SetMaterial (Variables|Default|GetEtat%20Poivron) 1 "/Game/Pizza/Models_3D/Garnitures/Poivrons/Poivron_R_Bruh.Poivron_R_Bruh")
  (Rendering|Material|SetMaterial (Variables|Default|GetEtat%20Poivron) 2 "/Game/Pizza/Models_3D/Garnitures/Poivrons/Poivron_J_Bruh.Poivron_J_Bruh")
  (Rendering|Material|SetMaterial (Variables|Default|GetEtat%20Poivron) 3 "/Game/Pizza/Models_3D/Garnitures/Poivrons/Poivron_B_Bruh.Poivron_B_Bruh")
  (Rendering|Material|SetMaterial (Variables|Default|GetEtat%20Poivron) 4 "/Game/Pizza/Models_3D/Garnitures/Poivrons/Poivron_V_Brulé.Poivron_V_Brulé")
  (Rendering|Material|SetMaterial (Variables|Default|GetEtat%20Poivron) 5 "/Game/Pizza/Models_3D/Garnitures/Poivrons/Poivron_B_Bruh.Poivron_B_Bruh")
  (Rendering|Material|SetMaterial (Variables|Debug|GetStaticMeshComponent) 0 "/Game/Pizza/Mat/MAT_Noir.MAT_Noir")
  (Rendering|Material|SetMaterial (Variables|Default|GetEtat%20Crevettes) 0 "/Game/Pizza/Models_3D/Garnitures/Crevettes/Mat_Crevette_Bruh.Mat_Crevette_Bruh")
  (Rendering|Material|SetMaterial (Variables|Default|GetEtat%20Crevettes) 1 "/Game/Pizza/Models_3D/Garnitures/Crevettes/Crevette2_Bruh.Crevette2_Bruh")
  (Rendering|Material|SetMaterial _etat_ver 1 "/Game/Pizza/Mat/MAT_Noir.MAT_Noir")
  (Rendering|Material|SetMaterial _etat_ver 2 "/Game/Pizza/Mat/MAT_Noir.MAT_Noir")
  (Rendering|Material|SetMaterial (Variables|Default|GetEtat%20Moisi) 0 "/Game/Pizza/Models_3D/Garnitures/Moisissure/Mat_Moisi_Bruh.Mat_Moisi_Bruh"))

(event EventDrop
  ;[1 1 1] PICKABLE
  (Physics|SetSimulatePhysics (Variables|Debug|GetStaticMeshComponent) true)
  (Transformation|DetachFromActor "KeepWorld" "KeepWorld" "KeepWorld"))

(event EventPickup
  (params (AttachTo :type Scene%20Component%20Object%20Reference))
  ;[1 1 1] PICKABLE
  (Physics|SetSimulatePhysics (Variables|Debug|GetStaticMeshComponent) false)
  (Transformation|AttachComponentToComponent (VehicleSound|GetRootComponent) AttachTo "None" "KeepWorld" "KeepWorld" "KeepWorld" false))

(event EventTick
  (params (DeltaSeconds :type Float%20%28single-precision%29))
  ;[0.5469 0.3331 0] Gestion de cuisson
  (if (Variables|Default|GetChauffe)
    (Variables|Default|SetEtat%20de%20chauffe (+ DeltaSeconds (Variables|Default|GetEtat%20de%20chauffe)))
    (if (>= (Variables|Default|GetEtat%20de%20chauffe) (Variables|Default|GetStade%20Cuisson%20Ok))
      (if (Variables|Default|GetCuite)
        (if (>= (Variables|Default|GetEtat%20de%20chauffe) (Variables|Default|GetStade%20Cuisson%20ratée)) :!label _label
          (if (not (Variables|Default|GetBrulée))
            (Variables|Default|SetBrulée true)
            (CallFunction|BRULE)
            (Variables|Default|SetCuite false)
            (if (>= (Variables|Default|GetEtat%20de%20chauffe) (Variables|Default|GetBRULURENFER))
              (if (not (Variables|Default|GetDESINTEGRATION))
                (Variables|Default|SetDESINTEGRATION true)
                (Actor|DestroyActor)))))
        (elif (not (Variables|Default|GetBrulée))
          (Variables|Default|SetCuite true)
          (CallFunction|CUIT)
          (goto _label))))))

(fn ConstructionScript)

(fn CheckOverlappObject
  (params (OverlapActor :type Actor%20Object%20Reference) (ClassName :type Name))
  (switch name ClassName))