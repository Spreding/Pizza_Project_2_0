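; BP_PU_Dépot is the pizza drop-off that grades delivered pizzas against five sequential orders.
; SelectionCommande shows the current order's BP_PU_Commande actor and arms the Box overlap check.
; Overlapping pizzas lose NOTE points per wrong topping or cooking flag; VerificationValeurPizza converts NOTE into result flags, then orders hide, the pizza is destroyed and the order advances.
; The fifth order's check repeats the order-4 condition, so it never runs.
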(event `Verification Valeur Pizza`
  ;[1 1 1] Addition N°3
  (if (== (`self.NOTE`) 3)
    (set `self.C'estOuiPourLesThunes 3/3` true)
    (elif (== (`self.NOTE`) 2)
      (set `self.C'estOuiPourLesThunes 2/3` true)
      (elif (== (`self.NOTE`) 1)
        (set `self.C'estOuiPourLesThunes 1/3` true)
        (elif (<= (`self.NOTE`) 0)
          (set `self.BAD` true))))))

(event `Reset All commands`
  ;[1 1 1] Reset commands 5/5
  (`self.Reset Commande 1`)
  (`self.Reset Commande 2`)
  (`self.Reset Commande 3`)
  (`self.Reset Commmande 4`)
  (`self.Reset Commande 5`))

(event `Reset Commande 1`
  ;[1 1 1] RESET COMMANDE 1
  (bind _outactors (`GameplayStatics.GetAllActorsOfClass` "/Game/Pizza/Blueprints/Commandes/BP_PU_Commande_1.BP_PU_Commande_1_C"))
  (for _array_element _outactors
    (`SceneComponent.SetVisibility` (`StaticMeshActor.StaticMeshComponent` _array_element) false true)
    (set `self.Ready to cook` false)))

(event `-1`
  ;[0 1 0.9191] Soustraction
  (set `self.NOTE` (- (`self.NOTE`) 1)))

(event `self.Box.OnComponentBeginOverlap`
  (params (OverlappedComponent :type "PrimitiveComponent Object Reference") (OtherActor :type "Actor Object Reference") (OtherComp :type "PrimitiveComponent Object Reference") (OtherBodyIndex :type Integer) (bFromSweep :type Boolean) (SweepResult :type "HitResult Structure (by ref)"))
  ;[1 1 1] CHECK
  (if (`self.Ready to cook`)
    (if (== (`GameplayStatics.GetObjectClass` OtherActor) "/Game/Pizza/Blueprints/BP_PU_Pizza.BP_PU_Pizza_C")
      (bind _outactors (`GameplayStatics.GetAllActorsOfClass` "/Game/Pizza/Blueprints/BP_PU_Pizza.BP_PU_Pizza_C"))
      (for _array_element _outactors
        (if (== _array_element OtherActor)
          (if (== (`self.N° De La Commande`) 1)
            (bind _asbp_pu_pizza (cast `/Game/Pizza/Blueprints/BP_PU_Pizza` _array_element))
            (set `self.Pizza ON Depot` true)
            (if (`/Game/Pizza/Blueprints/BP_PU_Pizza.Sauce 1` _asbp_pu_pizza)
              (`self.-1`))
            (if (`/Game/Pizza/Blueprints/BP_PU_Pizza.Sauce 2` _asbp_pu_pizza)
              (`self.-1`))
            (if (`/Game/Pizza/Blueprints/BP_PU_Pizza.Sauce 3` _asbp_pu_pizza)
              (`self.-1`))
            (if (`/Game/Pizza/Blueprints/BP_PU_Pizza.Sauce Niv3` _asbp_pu_pizza)
              (`self.-1`))
            (if (`/Game/Pizza/Blueprints/BP_PU_Pizza.Cuite` _asbp_pu_pizza)
              (`self.-1`))
            (if (`/Game/Pizza/Blueprints/BP_PU_Pizza.Brulée` _asbp_pu_pizza)
              (`self.-1`))
            (if (`/Game/Pizza/Blueprints/BP_PU_Pizza.Fromage` _asbp_pu_pizza)
              (`self.-1`))
            (if (`/Game/Pizza/Blueprints/BP_PU_Pizza.Champignon` _asbp_pu_pizza)
              (`self.-1`))
            (if (`/Game/Pizza/Blueprints/BP_PU_Pizza.Chorizo` _asbp_pu_pizza)
              (`self.-1`))
            (if (`/Game/Pizza/Blueprints/BP_PU_Pizza.Poivron` _asbp_pu_pizza)
              (`self.-1`))
            (if (`/Game/Pizza/Blueprints/BP_PU_Pizza.Crevettes` _asbp_pu_pizza)
              (`self.-1`))
            (if (`/Game/Pizza/Blueprints/BP_PU_Pizza.Dechet` _asbp_pu_pizza)
              (`self.-1`))
            (if (`/Game/Pizza/Blueprints/BP_PU_Pizza.Ver` _asbp_pu_pizza)
              (`self.-1`))
            (if (`/Game/Pizza/Blueprints/BP_PU_Pizza.Moisi` _asbp_pu_pizza)
              (`self.-1`))
            (if (`/Game/Pizza/Blueprints/BP_PU_Pizza.Savon` _asbp_pu_pizza)
              (`self.-1`))
            (set `self.Pizza ON Depot` true)
            (`self.Verification Valeur Pizza`)
            (`self.Reset All commands`)
            (set `self.NOTE` 3)
            (`self.K2_DestroyActor` _asbp_pu_pizza)
            (set `self.N° De La Commande` 2)
            (elif (== (`self.N° De La Commande`) 2)
              (bind _asbp_pu_pizza_2 (cast `/Game/Pizza/Blueprints/BP_PU_Pizza` _array_element))
              (set `self.Pizza ON Depot` true)
              (if (not (`/Game/Pizza/Blueprints/BP_PU_Pizza.Sauce 1` _asbp_pu_pizza_2))
                (`self.-1`))
              (if (`/Game/Pizza/Blueprints/BP_PU_Pizza.Sauce 2` _asbp_pu_pizza_2)
                (`self.-1`))
              (if (`/Game/Pizza/Blueprints/BP_PU_Pizza.Sauce 3` _asbp_pu_pizza_2)
                (`self.-1`))
              (if (not (`/Game/Pizza/Blueprints/BP_PU_Pizza.Sauce Niv3` _asbp_pu_pizza_2))
                (`self.-1`))
              (if (not (`/Game/Pizza/Blueprints/BP_PU_Pizza.Cuite` _asbp_pu_pizza_2))
                (`self.-1`))
              (if (`/Game/Pizza/Blueprints/BP_PU_Pizza.Brulée` _asbp_pu_pizza_2)
                (`self.-1`))
              (if (not (`/Game/Pizza/Blueprints/BP_PU_Pizza.Fromage` _asbp_pu_pizza_2))
                (`self.-1`))
              (if (not (`/Game/Pizza/Blueprints/BP_PU_Pizza.Champignon` _asbp_pu_pizza_2))
                (`self.-1`))
              (if (`/Game/Pizza/Blueprints/BP_PU_Pizza.Chorizo` _asbp_pu_pizza_2)
                (`self.-1`))
              (if (`/Game/Pizza/Blueprints/BP_PU_Pizza.Poivron` _asbp_pu_pizza_2)
                (`self.-1`))
              (if (`/Game/Pizza/Blueprints/BP_PU_Pizza.Crevettes` _asbp_pu_pizza_2)
                (`self.-1`))
              (if (`/Game/Pizza/Blueprints/BP_PU_Pizza.Dechet` _asbp_pu_pizza_2)
                (`self.-1`))
              (if (`/Game/Pizza/Blueprints/BP_PU_Pizza.Ver` _asbp_pu_pizza_2)
                (`self.-1`))
              (if (`/Game/Pizza/Blueprints/BP_PU_Pizza.Moisi` _asbp_pu_pizza_2)
                (`self.-1`))
              (if (`/Game/Pizza/Blueprints/BP_PU_Pizza.Savon` _asbp_pu_pizza_2)
                (`self.-1`))
              (set `self.Pizza ON Depot` true)
              (`self.Verification Valeur Pizza`)
              (`self.Reset All commands`)
              (set `self.NOTE` 3)
              (`self.K2_DestroyActor` _asbp_pu_pizza_2)
              (set `self.N° De La Commande` 3)
              (elif (== (`self.N° De La Commande`) 3)
                (bind _asbp_pu_pizza_3 (cast `/Game/Pizza/Blueprints/BP_PU_Pizza` _array_element))
                (set `self.Pizza ON Depot` true)
                (if (not (`/Game/Pizza/Blueprints/BP_PU_Pizza.Sauce 1` _asbp_pu_pizza_3))
                  (`self.-1`))
                (if (`/Game/Pizza/Blueprints/BP_PU_Pizza.Sauce 2` _asbp_pu_pizza_3)
                  (`self.-1`))
                (if (`/Game/Pizza/Blueprints/BP_PU_Pizza.Sauce 3` _asbp_pu_pizza_3)
                  (`self.-1`))
                (if (not (`/Game/Pizza/Blueprints/BP_PU_Pizza.Sauce Niv3` _asbp_pu_pizza_3))
                  (`self.-1`))
                (if (`/Game/Pizza/Blueprints/BP_PU_Pizza.Cuite` _asbp_pu_pizza_3)
                  (`self.-1`))
                (if (not (`/Game/Pizza/Blueprints/BP_PU_Pizza.Brulée` _asbp_pu_pizza_3))
                  (`self.-1`))
                (if (`/Game/Pizza/Blueprints/BP_PU_Pizza.Fromage` _asbp_pu_pizza_3)
                  (`self.-1`))
                (if (`/Game/Pizza/Blueprints/BP_PU_Pizza.Champignon` _asbp_pu_pizza_3)
                  (`self.-1`))
                (if (not (`/Game/Pizza/Blueprints/BP_PU_Pizza.Chorizo` _asbp_pu_pizza_3))
                  (`self.-1`))
                (if (not (`/Game/Pizza/Blueprints/BP_PU_Pizza.Poivron` _asbp_pu_pizza_3))
                  (`self.-1`))
                (if (`/Game/Pizza/Blueprints/BP_PU_Pizza.Crevettes` _asbp_pu_pizza_3)
                  (`self.-1`))
                (if (`/Game/Pizza/Blueprints/BP_PU_Pizza.Dechet` _asbp_pu_pizza_3)
                  (`self.-1`))
                (if (`/Game/Pizza/Blueprints/BP_PU_Pizza.Ver` _asbp_pu_pizza_3)
                  (`self.-1`))
                (if (`/Game/Pizza/Blueprints/BP_PU_Pizza.Moisi` _asbp_pu_pizza_3)
                  (`self.-1`))
                (if (`/Game/Pizza/Blueprints/BP_PU_Pizza.Savon` _asbp_pu_pizza_3)
                  (`self.-1`))
                (set `self.Pizza ON Depot` true)
                (`self.Verification Valeur Pizza`)
                (`self.Reset All commands`)
                (set `self.NOTE` 3)
                (`self.K2_DestroyActor` _asbp_pu_pizza_3)
                (set `self.N° De La Commande` 4)
                (elif (== (`self.N° De La Commande`) 4)
                  (bind _asbp_pu_pizza_4 (cast `/Game/Pizza/Blueprints/BP_PU_Pizza` _array_element))
                  (set `self.Pizza ON Depot` true)
                  (if (`/Game/Pizza/Blueprints/BP_PU_Pizza.Sauce 1` _asbp_pu_pizza_4)
                    (`self.-1`))
                  (if (not (`/Game/Pizza/Blueprints/BP_PU_Pizza.Sauce 2` _asbp_pu_pizza_4))
                    (`self.-1`))
                  (if (`/Game/Pizza/Blueprints/BP_PU_Pizza.Sauce 3` _asbp_pu_pizza_4)
                    (`self.-1`))
                  (if (not (`/Game/Pizza/Blueprints/BP_PU_Pizza.Sauce Niv3` _asbp_pu_pizza_4))
                    (`self.-1`))
                  (if (not (`/Game/Pizza/Blueprints/BP_PU_Pizza.Cuite` _asbp_pu_pizza_4))
                    (`self.-1`))
                  (if (`/Game/Pizza/Blueprints/BP_PU_Pizza.Brulée` _asbp_pu_pizza_4)
                    (`self.-1`))
                  (if (not (`/Game/Pizza/Blueprints/BP_PU_Pizza.Fromage` _asbp_pu_pizza_4))
                    (`self.-1`))
                  (if (`/Game/Pizza/Blueprints/BP_PU_Pizza.Champignon` _asbp_pu_pizza_4)
                    (`self.-1`))
                  (if (`/Game/Pizza/Blueprints/BP_PU_Pizza.Chorizo` _asbp_pu_pizza_4)
                    (`self.-1`))
                  (if (not (`/Game/Pizza/Blueprints/BP_PU_Pizza.Poivron` _asbp_pu_pizza_4))
                    (`self.-1`))
                  (if (not (`/Game/Pizza/Blueprints/BP_PU_Pizza.Crevettes` _asbp_pu_pizza_4))
                    (`self.-1`))
                  (if (`/Game/Pizza/Blueprints/BP_PU_Pizza.Dechet` _asbp_pu_pizza_4)
                    (`self.-1`))
                  (if (not (`/Game/Pizza/Blueprints/BP_PU_Pizza.Ver` _asbp_pu_pizza_4))
                    (`self.-1`))
                  (if (`/Game/Pizza/Blueprints/BP_PU_Pizza.Moisi` _asbp_pu_pizza_4)
                    (`self.-1`))
                  (if (`/Game/Pizza/Blueprints/BP_PU_Pizza.Savon` _asbp_pu_pizza_4)
                    (`self.-1`))
                  (set `self.Pizza ON Depot` true)
                  (`self.Verification Valeur Pizza`)
                  (`self.Reset All commands`)
                  (set `self.NOTE` 3)
                  (`self.K2_DestroyActor` _asbp_pu_pizza_4)
                  (set `self.N° De La Commande` 5)
                  (elif (== (`self.N° De La Commande`) 4)
                    (bind _asbp_pu_pizza_5 (cast `/Game/Pizza/Blueprints/BP_PU_Pizza` _array_element))
                    (set `self.Pizza ON Depot` true)
                    (if (`/Game/Pizza/Blueprints/BP_PU_Pizza.Sauce 1` _asbp_pu_pizza_5)
                      (`self.-1`))
                    (if (not (`/Game/Pizza/Blueprints/BP_PU_Pizza.Sauce 2` _asbp_pu_pizza_5))
                      (`self.-1`))
                    (if (`/Game/Pizza/Blueprints/BP_PU_Pizza.Sauce 3` _asbp_pu_pizza_5)
                      (`self.-1`))
                    (if (not (`/Game/Pizza/Blueprints/BP_PU_Pizza.Sauce Niv3` _asbp_pu_pizza_5))
                      (`self.-1`))
                    (if (`/Game/Pizza/Blueprints/BP_PU_Pizza.Cuite` _asbp_pu_pizza_5)
                      (`self.-1`))
                    (if (not (`/Game/Pizza/Blueprints/BP_PU_Pizza.Brulée` _asbp_pu_pizza_5))
                      (`self.-1`))
                    (if (`/Game/Pizza/Blueprints/BP_PU_Pizza.Fromage` _asbp_pu_pizza_5)
                      (`self.-1`))
                    (if (`/Game/Pizza/Blueprints/BP_PU_Pizza.Champignon` _asbp_pu_pizza_5)
                      (`self.-1`))
                    (if (`/Game/Pizza/Blueprints/BP_PU_Pizza.Chorizo` _asbp_pu_pizza_5)
                      (`self.-1`))
                    (if (`/Game/Pizza/Blueprints/BP_PU_Pizza.Poivron` _asbp_pu_pizza_5)
                      (`self.-1`))
                    (if (`/Game/Pizza/Blueprints/BP_PU_Pizza.Crevettes` _asbp_pu_pizza_5)
                      (`self.-1`))
                    (if (not (`/Game/Pizza/Blueprints/BP_PU_Pizza.Dechet` _asbp_pu_pizza_5))
                      (`self.-1`))
                    (if (`/Game/Pizza/Blueprints/BP_PU_Pizza.Ver` _asbp_pu_pizza_5)
                      (`self.-1`))
                    (if (not (`/Game/Pizza/Blueprints/BP_PU_Pizza.Moisi` _asbp_pu_pizza_5))
                      (`self.-1`))
                    (if (`/Game/Pizza/Blueprints/BP_PU_Pizza.Savon` _asbp_pu_pizza_5)
                      (`self.-1`))
                    (set `self.Pizza ON Depot` true)
                    (`self.Verification Valeur Pizza`)
                    (`self.Reset All commands`)
                    (set `self.NOTE` 3)
                    (`self.K2_DestroyActor` _asbp_pu_pizza_5)
                    (set `self.N° De La Commande` 5)))))))))))

(event `Reset Commande 2`
  (bind _outactors (`GameplayStatics.GetAllActorsOfClass` "/Game/Pizza/Blueprints/Commandes/BP_PU_Commande_2.BP_PU_Commande_2_C"))
  (for _array_element _outactors
    (`SceneComponent.SetVisibility` (`Actor.RootComponent` _array_element) false true)
    (set `self.Ready to cook` false)))

(event `Reset Commande 3`
  (bind _outactors (`GameplayStatics.GetAllActorsOfClass` "/Game/Pizza/Blueprints/Commandes/BP_PU_Commande_3.BP_PU_Commande_3_C"))
  (for _array_element _outactors
    (`SceneComponent.SetVisibility` (`Actor.RootComponent` _array_element) false true)
    (set `self.Ready to cook` false)))

(event `Reset Commmande 4`
  (bind _outactors (`GameplayStatics.GetAllActorsOfClass` "/Game/Pizza/Blueprints/Commandes/BP_PU_Commande_4.BP_PU_Commande_4_C"))
  (for _array_element _outactors
    (`SceneComponent.SetVisibility` (`Actor.RootComponent` _array_element) false true)
    (set `self.Ready to cook` false)))

(event `Reset Commande 5`
  (bind _outactors (`GameplayStatics.GetAllActorsOfClass` "/Game/Pizza/Blueprints/Commandes/BP_PU_Commande_5.BP_PU_Commande_5_C"))
  (for _array_element _outactors
    (`SceneComponent.SetVisibility` (`Actor.RootComponent` _array_element) false true)
    (set `self.Ready to cook` false)))

(event `self.Box.OnComponentEndOverlap`
  (params (OverlappedComponent :type "PrimitiveComponent Object Reference") (OtherActor :type "Actor Object Reference") (OtherComp :type "PrimitiveComponent Object Reference") (OtherBodyIndex :type Integer))
  ;[0 1 0.9665] Reset si commande est retiré.
  (bind _outactors (`GameplayStatics.GetAllActorsOfClass` "/Game/Pizza/Blueprints/BP_PU_Pizza.BP_PU_Pizza_C"))
  (for _array_element _outactors
    (if (== OverlappedComponent _array_element)
      (set `self.Pizza ON Depot` false)
      (set `self.NOTE` 3))))

(event `self.ReceiveBeginPlay`
  ;[1 1 1] BEGIN PLAY
  (set `self.N° De La Commande` 1)
  (`self.Reset All commands`))

(event `SelectionCommande`
  ;[1 0 0.01578] BOUTON PRESSED
  (bind _outactors (`GameplayStatics.GetAllActorsOfClass` "BP_PU_Dépot_C"))
  (for _array_element _outactors
    (bind `_asbp_pu_dépot` (cast `/Game/Pizza/Blueprints/BP_PU_Dépot` _array_element))
    (if (== (`/Game/Pizza/Blueprints/BP_PU_Dépot.N° De La Commande` `_asbp_pu_dépot`) 1)
      ;[1 0.0124 0] COMMANDE VISIBLE 1
      (bind _outactors_2 (`GameplayStatics.GetAllActorsOfClass` "/Game/Pizza/Blueprints/Commandes/BP_PU_Commande_1.BP_PU_Commande_1_C"))
      (for _array_element_2 _outactors_2
        (bind _asbp_pu_commande_1 (cast `/Game/Pizza/Blueprints/Commandes/BP_PU_Commande_1` _array_element_2))
        (`SceneComponent.SetVisibility` (`StaticMeshActor.StaticMeshComponent` _asbp_pu_commande_1) true true)
        (`SceneComponent.SetWorldScale3D` (`Actor.RootComponent` (`self.Fromage_Icon`)) (0.0 0.0 0.0))
        (set `self.Ready to cook` true))
      (elif (== (`/Game/Pizza/Blueprints/BP_PU_Dépot.N° De La Commande` `_asbp_pu_dépot`) 2)
        ;[1 0.4104 0] COMMANDE VISIBLE 2
        (bind _outactors_3 (`GameplayStatics.GetAllActorsOfClass` "/Game/Pizza/Blueprints/Commandes/BP_PU_Commande_2.BP_PU_Commande_2_C"))
        (for _array_element_3 _outactors_3
          (bind _asbp_pu_commande_2 (cast `/Game/Pizza/Blueprints/Commandes/BP_PU_Commande_2` _array_element_3))
          (`SceneComponent.SetVisibility` (`Actor.RootComponent` _asbp_pu_commande_2) true true)
          (set `self.Ready to cook` true))
        (elif (== (`/Game/Pizza/Blueprints/BP_PU_Dépot.N° De La Commande` `_asbp_pu_dépot`) 3)
          ;[1 0.9385 0] COMMANDE VISIBLE 3
          (bind _outactors_4 (`GameplayStatics.GetAllActorsOfClass` "/Game/Pizza/Blueprints/Commandes/BP_PU_Commande_3.BP_PU_Commande_3_C"))
          (for _array_element_4 _outactors_4
            (`SceneComponent.SetVisibility` (`Actor.RootComponent` _array_element_4) true true)
            (set `self.Ready to cook` true))
          (elif (== (`/Game/Pizza/Blueprints/BP_PU_Dépot.N° De La Commande` `_asbp_pu_dépot`) 4)
            ;[0 1 0.03511] COMMANDE VISIBLE 4
            (bind _outactors_5 (`GameplayStatics.GetAllActorsOfClass` "/Game/Pizza/Blueprints/Commandes/BP_PU_Commande_4.BP_PU_Commande_4_C"))
            (for _array_element_5 _outactors_5
              (`SceneComponent.SetVisibility` (`Actor.RootComponent` _array_element_5) true true)
              (set `self.Ready to cook` true))
            (elif (== (`/Game/Pizza/Blueprints/BP_PU_Dépot.N° De La Commande` `_asbp_pu_dépot`) 5)
              ;[0 0.1146 0.004022] COMMANDE VISIBLE 5
              (bind _outactors_6 (`GameplayStatics.GetAllActorsOfClass` "/Game/Pizza/Blueprints/Commandes/BP_PU_Commande_5.BP_PU_Commande_5_C"))
              (for _array_element_6 _outactors_6
                (`SceneComponent.SetVisibility` (`Actor.RootComponent` _array_element_6) true true)
                (set `self.Ready to cook` true))
              (elif (== (`/Game/Pizza/Blueprints/BP_PU_Dépot.N° De La Commande` `_asbp_pu_dépot`) 6)
                _))))))))

(fn `UserConstructionScript`)