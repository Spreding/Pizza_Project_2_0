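; Interactive buzzer button that is physically pushed down by whatever component overlaps it.
; The first overlapping component and its starting location are stored until that component leaves.
; Each Tick, its movement in the base mesh's local Z becomes a clamped press depth for the buzzer mesh, which resets through VInterpTo when released.
; It only handles the motion and fires no pressed event.
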(event `self.Mesh_Bouton_Buzzer.OnComponentBeginOverlap`
  (params (OverlappedComponent :type "PrimitiveComponent Object Reference") (OtherActor :type "Actor Object Reference") (OtherComp :type "PrimitiveComponent Object Reference") (OtherBodyIndex :type Integer) (bFromSweep :type Boolean) (SweepResult :type "HitResult Structure (by ref)"))
  (`/Engine/EditorBlueprintResources/StandardMacros.IsValid` (`self.Overlapped_Component`)
    (:`Is Not Valid`
      (bind _output_get (set `self.Overlapped_Component` OtherComp))
      (set `self.Initial_Overlap_Location` (`SceneComponent.K2_GetComponentLocation` _output_get)))))

(event `self.Mesh_Bouton_Buzzer.OnComponentEndOverlap`
  (params (OverlappedComponent :type "PrimitiveComponent Object Reference") (OtherActor :type "Actor Object Reference") (OtherComp :type "PrimitiveComponent Object Reference") (OtherBodyIndex :type Integer))
  (if (== OtherComp (`self.Overlapped_Component`))
    (set `self.Overlapped_Component` null)))

(event `self.ReceiveTick`
  (params (DeltaSeconds :type "Float (single-precision)"))
  (bind _mesh_bouton_buzzer (`self.Mesh_Bouton_Buzzer`))
  (bind _mesh_boutonbase (`self.Mesh_BoutonBase`))
  (bind (_returnvalue_x _returnvalue_y _returnvalue_z) (`KismetMathLibrary.BreakVector` (- (`KismetMathLibrary.InverseTransformLocation` (`SceneComponent.K2_GetComponentToWorld` _mesh_boutonbase) (`self.Initial_Overlap_Location`)) (`KismetMathLibrary.InverseTransformLocation` (`SceneComponent.K2_GetComponentToWorld` _mesh_boutonbase) (`SceneComponent.K2_GetComponentLocation` (`self.Overlapped_Component`))))))
  (`|ExecutionSequence`
    (:`then_0`
      (`/Engine/EditorBlueprintResources/StandardMacros.IsValid` (`self.Overlapped_Component`)
        (:`Is Valid`
          (bind _output_get (set `self.Button_Press_Amount` (`KismetMathLibrary.FClamp` _returnvalue_z 0.0 (`self.MaxButton_Press_Amount`))))
          (`SceneComponent.K2_SetRelativeLocation` _mesh_bouton_buzzer (`KismetMathLibrary.MakeVector` 0.0 0.0 (* _output_get -1.0)) false false))
        (:`Is Not Valid`
          (`SceneComponent.K2_SetRelativeLocation` _mesh_bouton_buzzer (`KismetMathLibrary.VInterpTo` (`SceneComponent.RelativeLocation` (`self.Mesh_Bouton_Buzzer`)) (0.0 0.0 0.0) DeltaSeconds) false false))))))

(fn `UserConstructionScript`)