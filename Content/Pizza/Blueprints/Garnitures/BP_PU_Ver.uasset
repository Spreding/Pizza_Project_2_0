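; BP_PU_Ver is a VR grabbable pizza topping that can be thrown in the trash.
; Pickup, called by BP_MotionController, disables mesh physics, attaches the actor to the given component and plays a grab sound.
; Drop re-enables physics and detaches it.
; When its mesh begins overlapping BP_Poubelle, it increments that bin's COMPTEURBOUFFE counter, then destroys itself after a short delay.
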(event OnComponentBeginOverlap(StaticMeshComponent)
  (params (OverlappedComponent :type Primitive%20Component%20Object%20Reference) (OtherActor :type Actor%20Object%20Reference) (OtherComp :type Primitive%20Component%20Object%20Reference) (OtherBodyIndex :type Integer) (bFromSweep :type Boolean) (SweepResult :type Hit%20Result%20Structure%20%28by%20ref%29))
  (bind _asbp_poubelle (Utilities|Casting|CastToBP_Poubelle OtherActor))
  (if (stale _bsuccess)
    (Variables|/Game/Pizza/Blueprints/Poubelle/BP_Poubelle.BP_Poubelle_C|SetCOMPTEUR%20BOUFFE _asbp_poubelle (+ (Variables|/Game/Pizza/Blueprints/Poubelle/BP_Poubelle.BP_Poubelle_C|GetCOMPTEUR%20BOUFFE _asbp_poubelle) 1))
    (Utilities|FlowControl|Delay 2.0)
    (Actor|DestroyActor)))

(event EventBeginPlay)

(event Collision|EventActorBeginOverlap
  (params (OtherActor :type Actor%20Object%20Reference)))

(event EventPickup
  (params (AttachTo :type Scene%20Component%20Object%20Reference))
  (Physics|SetSimulatePhysics (Variables|Debug|GetStaticMeshComponent) false)
  (Transformation|AttachComponentToComponent (VehicleSound|GetRootComponent) AttachTo "None" "KeepWorld" "KeepWorld" "KeepWorld" false)
  (Audio|PlaySound2D "/Game/Pizza/SONS/grab.grab" 1.0 1.0 0.0 0 0))

(event EventDrop
  (Physics|SetSimulatePhysics (Variables|Debug|GetStaticMeshComponent) true)
  (Transformation|DetachFromActor "KeepWorld" "KeepWorld" "KeepWorld"))

(fn ConstructionScript)