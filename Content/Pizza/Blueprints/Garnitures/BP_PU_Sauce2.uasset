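; BP_PU_Sauce2 is a grabbable sauce item for the pizza game, picked up with motion controllers.
; Pickup turns off physics, attaches it to the given component and plays a grab sound, while Drop restores physics and detaches it.
; Its Sphere overlap destroys the item when the other actor is a Suppr_Sauce, found by looping over all actors of that class rather than casting.
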(event `/Game/Pizza/Blueprints/Base/PickupActorInterface.Pickup`
  (params (AttachTo :type "SceneComponent Object Reference"))
  (`PrimitiveComponent.SetSimulatePhysics` (`self.StaticMeshComponent`) false)
  (`SceneComponent.K2_AttachToComponent` (`self.K2_GetRootComponent`) AttachTo "None" "KeepWorld" "KeepWorld" "KeepWorld" false)
  (`GameplayStatics.PlaySound2D` "/Game/Pizza/SONS/grab.grab" 1.0 1.0 0.0 null null))

(event `/Game/Pizza/Blueprints/Base/PickupActorInterface.Drop`
  (`PrimitiveComponent.SetSimulatePhysics` (`self.StaticMeshComponent`) true)
  (`self.K2_DetachFromActor` "KeepWorld" "KeepWorld" "KeepWorld"))

(event `self.Sphere.OnComponentBeginOverlap`
  (params (OverlappedComponent :type "PrimitiveComponent Object Reference") (OtherActor :type "Actor Object Reference") (OtherComp :type "PrimitiveComponent Object Reference") (OtherBodyIndex :type Integer) (bFromSweep :type Boolean) (SweepResult :type "HitResult Structure (by ref)"))
  (bind _outactors (`GameplayStatics.GetAllActorsOfClass` "/Game/Pizza/Blueprints/Garnitures/Suppr_Sauce.Suppr_Sauce_C"))
  (for _array_element _outactors
    (if (== _array_element OtherActor)
      (`self.K2_DestroyActor`))))

(fn `UserConstructionScript`)