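; Physical push button in the pizza game that flags the third sauce as ready to spawn when fully pressed.
; Tick converts the overlapping component's movement into clamped button-local Z depression, then eases the button back on release.
; A resettable DoOnce at full depth sets Sauce3SpawnOk, turns the material green and plays a click.
; Release plays a second sound and restores red; hand-feedback logic is unconnected.
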(event `self.ReceiveTick`
  (params (DeltaSeconds :type "Float (single-precision)"))
  (bind _button (`self.Button`))
  (bind (_returnvalue_x _returnvalue_y _returnvalue_z) (`KismetMathLibrary.BreakVector` (- (`KismetMathLibrary.InverseTransformDirection` (`SceneComponent.K2_GetComponentToWorld` _button) (`self.InitialOverlapLocation`)) (`KismetMathLibrary.InverseTransformDirection` (`SceneComponent.K2_GetComponentToWorld` _button) (`SceneComponent.K2_GetComponentLocation` (`self.OverlappedComponent`))))))
  (`/Engine/EditorBlueprintResources/StandardMacros.IsValid` (`self.OverlappedComponent`)
    (:`Is Valid`
      (bind _output_get (set `self.ButtonPressAmount` (`KismetMathLibrary.FClamp` _returnvalue_z 0.0 (`self.MaxButtonPress`))))
      (`SceneComponent.K2_SetRelativeLocation` (`self.Button`) (- (`self.ButtonInitialLocation`) (`KismetMathLibrary.MakeVector` 0.0 0.0 _output_get)) false false)
      (if (>= (`self.ButtonPressAmount`) (`self.MaxButtonPress`))
        (`/Engine/EditorBlueprintResources/StandardMacros.DoOnce` false :!label _label
          (:`Completed`
            (set `self.Sauce3 Spawn Ok` true)
            (`PrimitiveComponent.SetMaterial` (`self.Button`) 0 "/Game/Pizza/Mat/MAT_Vert.MAT_Vert")
            (`GameplayStatics.PlaySoundAtLocation` "/Game/Pizza/SONS/bouton1.bouton1" (stale `self.Button.OnComponentBeginOverlap` _output_get_2) (struct) 1.0 1.0 0.0 null null null)))
        (else
          (goto _label :!via `Reset`))))
    (:`Is Not Valid`
      (`SceneComponent.K2_SetRelativeLocation` (`self.Button`) (`KismetMathLibrary.VInterpTo` (`SceneComponent.RelativeLocation` (`self.Button`)) (`self.ButtonInitialLocation`) DeltaSeconds 10.0) false false)
      (`PrimitiveComponent.SetMaterial` (`self.Button`) 0 "/Game/Pizza/Mat/MAT_Rouge.MAT_Rouge"))))

(event `self.Button.OnComponentBeginOverlap`
  (params (OverlappedComponent :type "PrimitiveComponent Object Reference") (OtherActor :type "Actor Object Reference") (OtherComp :type "PrimitiveComponent Object Reference") (OtherBodyIndex :type Integer) (bFromSweep :type Boolean) (SweepResult :type "HitResult Structure (by ref)"))
  (`/Engine/EditorBlueprintResources/StandardMacros.IsValid` (`self.OverlappedComponent`)
    (:`Is Not Valid`
      (bind _output_get (set `self.OverlappedComponent` OtherComp))
      (bind _output_get_2 (set `self.InitialOverlapLocation` (`SceneComponent.K2_GetComponentLocation` _output_get))))))

(event `self.Button.OnComponentEndOverlap`
  (params (OverlappedComponent :type "PrimitiveComponent Object Reference") (OtherActor :type "Actor Object Reference") (OtherComp :type "PrimitiveComponent Object Reference") (OtherBodyIndex :type Integer))
  (if (== OtherComp (`self.OverlappedComponent`))
    (set `self.OverlappedComponent` null)
    (`MeshComponent.SetScalarParameterValueOnMaterials` (`self.Button`) "State" 0.0)
    (`GameplayStatics.PlaySoundAtLocation` "/Game/Pizza/SONS/bouton2.bouton2" (stale `self.Button.OnComponentBeginOverlap` _output_get_2) (struct) 1.0 1.0 0.0 null null null)))

(event `self.ReceiveBeginPlay`
  (set `self.ButtonInitialLocation` (`SceneComponent.RelativeLocation` (`self.Button`))))

(fn `UserConstructionScript`)