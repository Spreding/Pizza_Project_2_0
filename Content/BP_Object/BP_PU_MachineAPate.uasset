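; Pizza dough machine that turns water and flour cells into up to three units of dough.
; Each overlap sphere accepts its cell type while its available flag is set, sets that counter to three and destroys the cell.
; Matching counters set the dough stock, shown by colored indicator cubes; counter texts refresh on Tick.
; A button event spends one dough to spawn BP_PateAPizza, without decrementing ingredient counters or re-enabling intake.
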(event `self.Sphere_Eau.OnComponentBeginOverlap`
  (params (OverlappedComponent :type "PrimitiveComponent Object Reference") (OtherActor :type "Actor Object Reference") (OtherComp :type "PrimitiveComponent Object Reference") (OtherBodyIndex :type Integer) (bFromSweep :type Boolean) (SweepResult :type "HitResult Structure (by ref)"))
  ;[1 0.9511 0] Collision eau et Farine
  (if (== (`GameplayStatics.GetObjectClass` OtherActor) "/Game/BP_Object/BP_PU_Cellule_Eau.BP_PU_Cellule_Eau_C")
    (if (`self.Stock Eau Disponible`)
      (`PrimitiveComponent.SetMaterial` (`self.Cube Etat Eau`) 0 "/Game/Pizza/Mat/MAT_Vert.MAT_Vert")
      (set `self.Stock Eau Disponible` false)
      (set `self.Compteur_Eau_Stock` 3)
      (`KismetSystemLibrary.Delay` 0.3)
      (`self.SetStockPates`)
      (`self.K2_DestroyActor` OtherActor))))

(event `self.Sphere_Farine.OnComponentBeginOverlap`
  (params (OverlappedComponent :type "PrimitiveComponent Object Reference") (OtherActor :type "Actor Object Reference") (OtherComp :type "PrimitiveComponent Object Reference") (OtherBodyIndex :type Integer) (bFromSweep :type Boolean) (SweepResult :type "HitResult Structure (by ref)"))
  ;[1 0.9511 0] Collision eau et Farine
  (if (== (`GameplayStatics.GetObjectClass` OtherActor) "/Game/BP_Object/BP_PU_Cellule_Farine.BP_PU_Cellule_Farine_C")
    (if (`self.Stock Farine Disponible`)
      (`PrimitiveComponent.SetMaterial` (`self.Cube Etat Farine`) 0 "/Game/Pizza/Mat/MAT_Vert.MAT_Vert")
      (set `self.Stock Farine Disponible` false)
      (set `self.Compteur_Farine_Stock` 3)
      (`KismetSystemLibrary.Delay` 0.3)
      (`self.SetStockPates`)
      (`self.K2_DestroyActor` OtherActor))))

(event `SetStockPates`
  (if (and (== (`self.Compteur_Eau_Stock`) 1) (== (`self.Compteur_Farine_Stock`) 1))
    (set `self.Stock Pate` 1)
    (elif (and (== (`self.Compteur_Eau_Stock`) 2) (== (`self.Compteur_Farine_Stock`) 2))
      (set `self.Stock Pate` 2)
      (elif (and (== (`self.Compteur_Eau_Stock`) 3) (== (`self.Compteur_Farine_Stock`) 3))
        (set `self.Stock Pate` 3))))
  (`self.CheckStockPates`))

(event `self.ReceiveTick`
  (params (DeltaSeconds :type "Float (single-precision)"))
  (`self.Update_Text_Eau`)
  (`self.Update_Text_Farine`))

(event `CheckStockPates`
  (for (_array_element _array_index) (`|MakeArray` (`self.Cube Etat 1 Pate`) (`self.Cube Etat 2 Pate`) (`self.Cube Etat 3 Pate`))
    (if (< _array_index (`self.Stock Pate`))
      (`PrimitiveComponent.SetMaterial` _array_element 0 "/Game/Pizza/Mat/MAT_Vert.MAT_Vert")
      (else
        (`PrimitiveComponent.SetMaterial` _array_element 0 "/Game/Pizza/Mat/MAT_Rouge.MAT_Rouge")))))

(event `PressionBoutonMachinePate`
  ;[1 1 1] SORTIE PIZZA BOUTON
  (if (>= (`self.Stock Pate`) 1)
    (set `self.Launch Pizza` true)
    (set `self.Stock Pate` (- (`self.Stock Pate`) 1))
    (`KismetSystemLibrary.PrintString` "SPAWN" true true (struct :`R` 0.165616 :`B` 1.0 :`A` 1.0))
    (`|SpawnActorFromClass` "/Game/BP_Object/BP_PateAPizza.BP_PateAPizza_C" (`KismetMathLibrary.MakeTransform` (`SceneComponent.K2_GetComponentLocation` (`self.StaticMesh`)) (struct) (0.02 0.02 0.02)) "Undefined" "OverrideRootScale" null null)
    (`self.CheckStockPates`)
    (set `self.Launch Pizza` false)))

(fn `Update_Text_Eau`
  (`TextRenderComponent.K2_SetText` (`self.Text_Count_Eau`) (`KismetTextLibrary.Conv_IntToText` (`self.Compteur_Eau_Stock`))))

(fn `Update_Text_Farine`
  (`TextRenderComponent.K2_SetText` (`self.Text_Count_Farine`) (`KismetTextLibrary.Conv_IntToText` (`self.Compteur_Farine_Stock`))))

(fn `UserConstructionScript`)