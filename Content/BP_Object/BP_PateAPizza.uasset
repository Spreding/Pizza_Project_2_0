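; Pizza dough actor that collects toppings and one sauce to build a pizza.
; Base hits identify ingredients by exact display name, then destroy each new one and either reveal its component or add a mesh; Champi reuses the Chorizo mesh.
; Boolean flags block duplicate hit toppings and make the three sauces mutually exclusive, each swapping the SauceTomate material.
; Sauce, secret ingredient and Vers events are not triggered within this graph.
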(event `self.Base.OnComponentHit`
  (params (HitComponent :type "PrimitiveComponent Object Reference") (OtherActor :type "Actor Object Reference") (OtherComp :type "PrimitiveComponent Object Reference") (NormalImpulse :type "Vector Structure") (Hit :type "HitResult Structure (by ref)"))
  (bind _returnvalue (`KismetSystemLibrary.GetDisplayName` OtherActor))
  (if (`KismetStringLibrary.EqualEqual_StrStr` _returnvalue "BP_Chorizo")
    (if (not (`self.haveChorizo`))
      (`self.setChorizo` OtherActor))
    (elif (`KismetStringLibrary.EqualEqual_StrStr` _returnvalue "BP_Champi")
      (if (not (`self.haveChampi`))
        (`self.setChampi` OtherActor))
      (elif (`KismetStringLibrary.EqualEqual_StrStr` _returnvalue "BP_Crevette")
        (if (not (`self.haveCrevette`))
          (`self.setCrevette` OtherActor))
        (elif (`KismetStringLibrary.EqualEqual_StrStr` _returnvalue "BP_Fromage")
          (if (not (`self.haveFromage`))
            (`self.setFromage` OtherActor))
          (elif (`KismetStringLibrary.EqualEqual_StrStr` _returnvalue "BP_Moisissure")
            (if (not (`self.haveMoisissure`))
              (`self.setMoisissure` OtherActor))
            (elif (`KismetStringLibrary.EqualEqual_StrStr` _returnvalue "BP_Poivron")
              (if (not (`self.havePoivron`))
                (`self.setPoivron` OtherActor)))))))))

(event `setTomatoSauce`
  ;[1 1 1] SET SAUCE
  (if (`self.haveTomatoSauce`)
    _
    (elif (not (or (`self.haveAlienSauce`) (`self.haveFromageSauce`)))
      (set `self.haveTomatoSauce` true)
      (`PrimitiveComponent.SetMaterial` (`self.Sauce_Tomate`) 0 "/Game/Pizza/Models_3D/Garnitures/Sauces/MAT_Sauce1_Froide.MAT_Sauce1_Froide"))))

(event `setAlienSauce`
  ;[1 1 1] SET SAUCE
  (if (`self.haveAlienSauce`)
    _
    (elif (not (or (`self.haveTomatoSauce`) (`self.haveFromageSauce`)))
      (set `self.haveAlienSauce` true)
      (`PrimitiveComponent.SetMaterial` (`self.Sauce_Tomate`) 0 "/Game/Pizza/Models_3D/Garnitures/Sauces/MAT_Sauce2_Froide.MAT_Sauce2_Froide"))))

(event `setFromageSauce`
  ;[1 1 1] SET SAUCE
  (if (`self.haveFromageSauce`)
    _
    (elif (not (or (`self.haveAlienSauce`) (`self.haveTomatoSauce`)))
      (set `self.haveFromageSauce` true)
      (`PrimitiveComponent.SetMaterial` (`self.Sauce_Tomate`) 0 "/Game/Pizza/Models_3D/Garnitures/Sauces/MAT_Sauce3_Froide.MAT_Sauce3_Froide"))))

(event `setSecretIngredient`
  (params (Actor :type "Actor Object Reference"))
  (`self.K2_DestroyActor` Actor)
  (`KismetSystemLibrary.PrintString` "Transformation")
  (set `self.haveSecretIngredient` true)
  (bind _returnvalue (`AddComponent|NODE_AddStaticMeshComponent-1`))
  (`StaticMeshComponent.SetStaticMesh` _returnvalue "/Game/Assets/3D/Pizza_Moisissure_Pizza.Pizza_Moisissure_Pizza"))

(event `setChampi`
  (params (Actor :type "Actor Object Reference"))
  (`self.K2_DestroyActor` Actor)
  (`KismetSystemLibrary.PrintString` "Transformation")
  (set `self.haveChampi` true)
  (bind _returnvalue (`AddComponent|NODE_AddStaticMeshComponent-2`))
  (`StaticMeshComponent.SetStaticMesh` _returnvalue "/Game/Assets/3D/Pizza_Chorizo_Pizza.Pizza_Chorizo_Pizza"))

(event `setChorizo`
  (params (Actor :type "Actor Object Reference"))
  (`self.K2_DestroyActor` Actor)
  (`KismetSystemLibrary.PrintString` "Transformation")
  (set `self.haveChorizo` true)
  (bind _returnvalue (`AddComponent|NODE_AddStaticMeshComponent-0`))
  (`StaticMeshComponent.SetStaticMesh` _returnvalue "/Game/Assets/3D/Pizza_Chorizo_Pizza.Pizza_Chorizo_Pizza"))

(event `setCrevette`
  (params (Actor :type "Actor Object Reference"))
  (set `self.haveCrevette` true)
  (`SceneComponent.SetVisibility` (`self.Crevette_Ingredient`) true false)
  (`self.K2_DestroyActor` Actor))

(event `setFromage`
  (params (Actor :type "Actor Object Reference"))
  (set `self.haveFromage` true)
  (`SceneComponent.SetVisibility` (`self.Fromage_Ingredient`) true false)
  (`self.K2_DestroyActor` Actor))

(event `setPoivron`
  (params (Actor :type "Actor Object Reference"))
  (set `self.havePoivron` true)
  (`SceneComponent.SetVisibility` (`self.Poivron_Ingredient`) true false)
  (`self.K2_DestroyActor` Actor))

(event `setMoisissure`
  (params (Actor :type "Actor Object Reference"))
  (set `self.haveMoisissure` true)
  (`SceneComponent.SetVisibility` (`self.Moisissure_Ingredient`) true false)
  (`self.K2_DestroyActor` Actor))

(event `setVers`
  (params (Actor :type "Actor Object Reference"))
  (set `self.haveVers` true)
  (`SceneComponent.SetVisibility` (`self.Vers_Ingredient`) true false)
  (`self.K2_DestroyActor` Actor))

(fn `UserConstructionScript`)